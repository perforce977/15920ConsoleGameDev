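; Player character Blueprint for the blue-haired girl, handling movement, camera look, jumping, lock-on and combo melee attacks.
; Holding lock-on finds the nearest EnemyMOTHA, eases control rotation toward it, moves a LockIN_Actor marker above it and sets a motion-warp target near it.
; Attacks play montages by combo index, with notifies reopening input, resetting the combo and toggling DamageBox collision.
; DamageBox overlaps apply damage calculated by the Stats component.
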(event OnComponentBeginOverlap(DamageBox)
  (params (OverlappedComponent :type Primitive%20Component%20Object%20Reference) (OtherActor :type Actor%20Object%20Reference) (OtherComp :type Primitive%20Component%20Object%20Reference) (OtherBodyIndex :type Integer) (bFromSweep :type Boolean) (SweepResult :type Hit%20Result%20Structure%20%28by%20ref%29))
  ;[0.15 0.15 0.15 0.5] Overlap Damage Definition
  (bind _damagedefined (Default|DefineDamage (Variables|Default|GetStats)))
  (Game|Damage|ApplyDamage OtherActor _damagedefined 0 0))

(event Input|EnhancedActionEvents|EnhancedInputActionLockIN
  (params (ActionValue :type Boolean) (ElapsedSeconds :type Float%20%28double-precision%29) (TriggeredSeconds :type Float%20%28double-precision%29) (InputAction :type Input%20Action%20Object%20Reference :default "/Game/Inputs/LockIN.LockIN"))
  ;[0.15 0.15 0.15 0.5] Lock In
  (:Triggered
    (bind _thenearestenemy (Variables|Default|GetTheNearestEnemy)
      (:then
        (Pawn|SetControlRotation (Game|GetPlayerController 0) (Math|Rotator|Lerp(Rotator) (Pawn|GetControlRotation (Game|GetPlayerController 0) :!class /Script/Engine.Controller) (Math|Rotator|FindLookatRotation (Transformation|GetActorLocation) (Transformation|GetActorLocation _thenearestenemy)) 0.03 true))
        (bind _thenearestenemy_2 (Variables|Default|GetTheNearestEnemy)
          (:then
            (bind _returnvalue (Actor|GetActorOfClass "/Game/Blueprints/LockIN_Actor.LockIN_Actor_C")) ; Only works when Actor is already present in Scene
            (bind _output_get (Variables|Default|SetMeThe_LockIN_Guy _returnvalue))
            (Transformation|SetActorLocation _output_get (+ (Transformation|GetActorLocation _thenearestenemy_2) "0.000000,0.000000,100.000000") false false))
          (:else)))
      (:else)))
  (:Started
    (CallFunction|FindDaNearestEyenemy)
    (Class|MotionWarpingComponent|AddorUpdateWarpTargetfromLocation (Variables|Default|GetMotionWarping) "Sacrifices" (+ (* (Math|Vector|GetUnitDirection(Vector) (Transformation|GetActorLocation (Variables|Default|GetTheNearestEnemy)) (Transformation|GetActorLocation)) (Variables|Default|GettheLerper)) (Transformation|GetActorLocation (Variables|Default|GetTheNearestEnemy)))) ; Causes a Mouse or Controller to be necessary, rather than just a touchpad
  )
  (:Completed
    (Variables|/Script/Engine.CharacterMovementComponent|SetbOrientRotationToMovement (Variables|Character|GetCharacterMovement) true)
    (Class|MotionWarpingComponent|RemoveWarpTarget (Variables|Default|GetMotionWarping) "Sacrifices")))

(event Input|EnhancedActionEvents|EnhancedInputActionWASD
  (params (ActionValue :type Vector%202D%20Structure) (ElapsedSeconds :type Float%20%28double-precision%29) (TriggeredSeconds :type Float%20%28double-precision%29) (InputAction :type Input%20Action%20Object%20Reference :default "/Game/Inputs/WASD.WASD"))
  (bind _returnvalue (Input|EnhancedActionValues|GetWASD))
  ;[0.15 0.15 0.15 0.5] Movement Basic
  (Pawn|Input|AddMovementInput (Transformation|GetActorForwardVector (Pawn|GetController)) (.x _returnvalue) false)
  (Pawn|Input|AddMovementInput (Transformation|GetActorRightVector (Pawn|GetController)) (.y _returnvalue) false))

(event Input|EnhancedActionEvents|EnhancedInputActionMouseMove
  (params (ActionValue :type Vector%202D%20Structure) (ElapsedSeconds :type Float%20%28double-precision%29) (TriggeredSeconds :type Float%20%28double-precision%29) (InputAction :type Input%20Action%20Object%20Reference :default "/Game/Inputs/MouseMove.MouseMove"))
  ;[0.15 0.15 0.15 0.5] Movement Basic
  (Pawn|Input|AddControllerYawInput (.x ActionValue))
  (Pawn|Input|AddControllerPitchInput (* (.y ActionValue) -1.0)))

(event Input|EnhancedActionEvents|EnhancedInputActionJump
  (params (ActionValue :type Boolean) (ElapsedSeconds :type Float%20%28double-precision%29) (TriggeredSeconds :type Float%20%28double-precision%29) (InputAction :type Input%20Action%20Object%20Reference :default "/Game/Inputs/Jump.Jump"))
  ;[0.15 0.15 0.15 0.5] Movement Basic
  (:Started
    (Character|Jump)))

(event Input|EnhancedActionEvents|EnhancedInputActionAttack
  (params (ActionValue :type Boolean) (ElapsedSeconds :type Float%20%28double-precision%29) (TriggeredSeconds :type Float%20%28double-precision%29) (InputAction :type Input%20Action%20Object%20Reference :default "/Game/Inputs/Attack.Attack"))
  (bind _damagebox (Variables|Default|GetDamageBox))
  ;[0.15 0.15 0.15 0.5] Attacking
  (:Started
    (if (Variables|Default|GetcanAttack)
      (Variables|Default|SetcanAttack false)
      (bind _notifyname (Animation|Montage|PlayMontage (Variables|Character|GetMesh) (Utilities|Select :Index (Variables|Default|GetComboIndex) :Option%200 "/Game/Characters/PlayerModelGirl/Anims/Attack1_Montage.Attack1_Montage" :Option%201 "/Game/Characters/PlayerModelGirl/Anims/Attack2_Montage.Attack2_Montage" :Option%202 "/Game/Characters/PlayerModelGirl/Anims/Attack3_Montage.Attack3_Montage"))
        (:then
          (Math|Integer|IncrementInt (Variables|Default|GetComboIndex)
            (:%20%20
              (if (> (Variables|Default|GetComboIndex) 3)
                (Variables|Default|SetComboIndex 0)))))
        (:OnNotifyBegin
          (switch name _notifyname
            (:YesNewAttack
              (Variables|Default|SetcanAttack true))
            (:ResetCombo
              (Variables|Default|SetComboIndex 0))
            (:DamageBoxACTIVE
              (Collision|SetCollisionEnabled _damagebox "QueryOnly"))))
        (:OnNotifyEnd
          (Collision|SetCollisionEnabled _damagebox "NoCollision"))))))

(fn ConstructionScript)

(fn FindDaNearestEyenemy
  (bind _outactors (Actor|GetAllActorsOfClass "/Game/Characters/Enemies/EnemyMOTHA.EnemyMOTHA_C"))
  (Variables|Default|SetTheNearestEnemy (.ReturnValue (Actor|FindNearestActor (Transformation|GetActorLocation) _outactors)))
  (Variables|/Script/Engine.CharacterMovementComponent|SetbOrientRotationToMovement (Variables|Character|GetCharacterMovement) false))